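; Throwable item Blueprint that serves as a distraction to lure enemies to where it lands.
; ThrowbyCharacter applies an impulse to the mesh, waits a fixed delay, then calls AttractEnemy.
; AttractEnemy sends the mesh's current location through GoTo to every actor implementing HandInterface.
; Item interface getters supply an item type and hint icon, while the grab, rope and hint text functions return empty or false defaults.
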(event Custom|AttractEnemy
  (bind _outactors (Actor|GetAllActorswithInterface "/Game/Roberto/Enemy/EnemyHand/HandInterface.HandInterface_C"))
  (for _array_element _outactors
    (Class|HandInterface|Goto(Message) _array_element (Transformation|GetWorldLocation (Variables|Default|GetMesh)))))

(event Collision|EventActorBeginOverlap
  (params (OtherActor :type Actor%20Object%20Reference)))

(event EventTick
  (params (DeltaSeconds :type Float%20%28single-precision%29)))

(event EventThrowbyCharacter
  (params (Force :type Vector :default "0, 0, 0"))
  (Physics|AddImpulse (Variables|Default|GetMesh) Force "None" false)
  (Utilities|FlowControl|Delay 2.0)
  (CallFunction|AttractEnemy))

(fn ConstructionScript)

(fn GetGrabBox
  (return 0))

(fn GetHintButtonIcon
  (return "NewEnumerator0"))

(fn GetHintUIText
  (return ""))

(fn GetItemType
  (return "NewEnumerator3"))

(fn GetRope
  (return 0))

(fn IsGrabbed?
  (return false))

(fn ReadytobeGrabbed?
  (return false))