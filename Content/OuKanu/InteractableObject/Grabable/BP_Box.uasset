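; BP_Box is a grabbable interactable box whose hint text offers climbing or grabbing.
; Grab and drop events nudge the mesh up or down one unit and set the grabbed flag.
; Getter functions expose itself, item type, state and a state-dependent button icon, while ReadyToBeGrabbed always returns false.
; It caches the player and its start location on BeginPlay, and ResetPosition sweeps and teleports it back there.
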(event Custom|ResetPosition
  (Transformation|SetWorldLocation (Variables|Default|Getboxmesh) (Variables|Default|GetStartLocation) true true))

(event EventBeginPlay
  (Variables|Default|SetStartLocation (Transformation|GetWorldLocation (Variables|Default|Getboxmesh)))
  (bind _returnvalue (Actor|GetActorOfClass "/Game/OuKanu/Character/BP_Player.BP_Player_C"))
  (Variables|Default|Setplayer _returnvalue))

(event EventGrabbyCharacter
  (params (Grab :type Boolean) (TargetComponent :type Scene%20Component%20Object%20Reference) (MeshComponent :type Mesh%20Component%20Object%20Reference))
  (bind _boxmesh (Variables|Default|Getboxmesh))
  (if Grab
    (Transformation|SetWorldLocation _boxmesh (+ (Transformation|GetWorldLocation _boxmesh) "0, 0,1.000000") false false)
    (Variables|Default|SetIsGrabbed true)
    (else
      (CallFunction|DropbyCharacter))))

(event EventDropbyCharacter
  (bind _boxmesh (Variables|Default|Getboxmesh))
  (Transformation|SetWorldLocation _boxmesh (+ (Transformation|GetWorldLocation _boxmesh) "0, 0,-1.000000") false false)
  (Variables|Default|SetIsGrabbed false))

(fn ConstructionScript)

(fn GetGrabBox
  (return self))

(fn GetHintButtonIcon
  (bind _isgrabbed (CallFunction|IsGrabbed?))
  (if _isgrabbed
    (return "NewEnumerator0")
    (else
      (return "NewEnumerator10"))))

(fn GetHintUIText
  (return "Press \"Space/A\" To Climb 
Press \"RightMouse/R2\"To Grab"))

(fn GetItemType
  (return "NewEnumerator1"))

(fn GetRope
  (return 0))

(fn IsGrabbed?
  (return (Variables|Default|GetIsGrabbed)))

(fn ReadytobeGrabbed?
  (return false))