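; BP_Bottle is a grabbable bottle that a character can pick up, drop, throw and destroy.
; Grabbing teleports it to the target component and switches constraint mode and collision profile; dropping reverts them with short delays before it is grabbable again.
; Throwing applies a velocity-change impulse, reset returns the mesh to its BeginPlay location, and destruction spawns a hit effect.
; Query functions report grab state, readiness, item type and a state-dependent hint icon.
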(event Custom|ResetPosition
  ;[1 1 1] Save & Load
  (Transformation|SetWorldLocation (Variables|Default|GetBottleMesh) (Variables|Default|GetStartLocation) true true)
  (Variables|Default|SetIsReady true))

(event EventBeginPlay
  ;[1 1 1] Save & Load
  (Variables|Default|SetStartLocation (Transformation|GetWorldLocation (Variables|Default|GetBottleMesh))))

(event EventGrabbyCharacter
  (params (Grab :type Boolean) (TargetComponent :type Scene%20Component%20Object%20Reference) (MeshComponent :type Mesh%20Component%20Object%20Reference))
  (bind _bottlemesh (Variables|Default|GetBottleMesh))
  (if Grab
    (Transformation|SetActorLocationAndRotation (Transformation|GetWorldLocation TargetComponent) "0, 0, 0" false true)
    (Class|PrimitiveComponent|SetConstraintMode _bottlemesh "Default")
    (Collision|SetCollisionProfileName _bottlemesh "PickableitemPicked" :!class /Script/Engine.PrimitiveComponent)
    (Variables|Default|SetIsGrabbed true)
    (Variables|Default|SetIsReady false)
    (Default|CallOnGrabEvent)
    (else
      (CallFunction|DropbyCharacter))))

(event EventDestructItem
  ;[1 1 1] VFX
  (Effects|SpawnEmitteratLocation "/Game/OuKanu/FX/FXVarietyPack/Particles/P_ky_hit1.P_ky_hit1" (Transformation|GetWorldLocation (Variables|Default|GetBottleMesh)))
  (Actor|DestroyActor))

(event EventDropbyCharacter
  (bind _bottlemesh (Variables|Default|GetBottleMesh))
  (Utilities|FlowControl|Delay 0.2)
  (Class|PrimitiveComponent|SetConstraintMode _bottlemesh "None")
  (Collision|SetCollisionProfileName _bottlemesh "PickableitemDefalut" :!class /Script/Engine.PrimitiveComponent)
  (Variables|Default|SetIsGrabbed false)
  (Utilities|FlowControl|Delay 0.5)
  (Variables|Default|SetIsReady true))

(event EventThrowbyCharacter
  (params (Force :type Vector :default "0, 0, 0"))
  (Physics|AddImpulse (Variables|Default|GetBottleMesh) Force "None" true))

(fn ConstructionScript)

(fn GetGrabBox
  (return 0))

(fn GetHintButtonIcon
  (if (Variables|Default|GetIsGrabbed)
    (return "NewEnumerator0")
    (else
      (return "NewEnumerator10"))))

(fn GetHintUIText
  (return ""))

(fn GetItemType
  (return "NewEnumerator0"))

(fn GetRope
  (return 0))

(fn IsGrabbed?
  (return (Variables|Default|GetIsGrabbed)))

(fn ReadytobeGrabbed?
  (return (Variables|Default|GetIsReady)))