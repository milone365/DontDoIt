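; DustExplosionBP is a short-lived damage volume, apparently the dust explosion of the Grount enemy.
; INIT stores a passed-in actor, caches all actors implementing BPI_Character, then after a one-second delay destroys both that actor and itself.
; When an actor begins overlapping the Cube and matches one in the cached list, it receives a HurtMessage with fixed damage.
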(event OnComponentBeginOverlap(Cube)
  (params (OverlappedComponent :type Primitive%20Component%20Object%20Reference) (OtherActor :type Actor%20Object%20Reference) (OtherComp :type Primitive%20Component%20Object%20Reference) (OtherBodyIndex :type Integer) (bFromSweep :type Boolean) (SweepResult :type Hit%20Result%20Structure%20%28by%20ref%29))
  (for _array_element (Variables|Default|GetTragets)
    (if (== _array_element OtherActor)
      (Class|BPICharacter|Hurt(Message) OtherActor 3e+01))))

(event Custom|INIT
  (params (NewParam :type Actor%20Object%20Reference))
  (Variables|Default|SetactorTodestroy NewParam)
  (bind _outactors (Actor|GetAllActorswithInterface "/Game/OuKanu/BP/Interface/BPI_Character.BPI_Character_C"))
  (Variables|Default|SetTragets _outactors)
  (Utilities|FlowControl|Delay 1.0)
  (Actor|DestroyActor (Variables|Default|GetactorTodestroy))
  (Actor|DestroyActor))

(fn ConstructionScript)