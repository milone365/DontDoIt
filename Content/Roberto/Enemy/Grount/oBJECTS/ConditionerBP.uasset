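; ConditionerBP is a throwable bottle actor that damages the GrountBP enemy on contact.
; ThrowbyCharacter enables physics on the bottle mesh and launches it along the player pawn's forward vector, scaled by Force, with a fixed upward boost.
; When its Box overlaps a GrountBP, it calls TakeDamage on the enemy, spawns an explosion, calls PickOff on BP_Player and destroys itself.
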(event OnComponentBeginOverlap(Box)
  (params (OverlappedComponent :type Primitive%20Component%20Object%20Reference) (OtherActor :type Actor%20Object%20Reference) (OtherComp :type Primitive%20Component%20Object%20Reference) (OtherBodyIndex :type Integer) (bFromSweep :type Boolean) (SweepResult :type Hit%20Result%20Structure%20%28by%20ref%29))
  (bind _asgrount_bp (Utilities|Casting|CastToGrountBP OtherActor))
  (Utilities|IsValid _asgrount_bp
    (:Is%20Valid
      (Default|TakeDamage _asgrount_bp)
      (Effects|SpawnEmitteratLocation "/Game/OuKanu/FX/FXVarietyPack/Particles/P_ky_explosion.P_ky_explosion" (Transformation|GetWorldLocation (Variables|Default|GetBottleMesh)))
      (bind _returnvalue (Actor|GetActorOfClass "/Game/OuKanu/Character/BP_Player.BP_Player_C"))
      (Default|PickOff _returnvalue)
      (Actor|DestroyActor))))

(event EventBeginPlay
  (|CallParentFunction) ; This node is disabled and will not be called.\nDrag off pins to build functionality.
)

(event Collision|EventActorBeginOverlap
  (params (OtherActor :type Actor%20Object%20Reference)))

(event EventTick
  (params (DeltaSeconds :type Float%20%28single-precision%29)))

(event EventThrowbyCharacter
  (params (Force :type Vector :default "0, 0, 0"))
  (bind _bottlemesh (Variables|Default|GetBottleMesh))
  (Physics|SetSimulatePhysics _bottlemesh true)
  (Physics|AddImpulse _bottlemesh (+ (* (Math|Vector|GetForwardVector (Variables|/Script/Engine.Actor|GetRootComponent (Game|Player|GetPlayerPawn 0))) (Variables|Default|GetForce)) "0, 0,1500.000000") "None" false))

(fn ConstructionScript
  (|CallParentFunction))