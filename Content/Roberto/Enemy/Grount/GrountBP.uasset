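; Boss enemy Grount, which fights the player with melee attacks, grab-and-throw swings and thrown rocks.
; Tick faces the player and runs a cooldown, choosing non-repeating random melee montages up close or rock-throw bursts with rests at range.
; Hand and foot overlap boxes deal damage or catch the player, who follows the hand socket until release.
; Battle end flags death on the animator, plays a level sequence and spawns a replacement actor.
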(event Custom|AntennaEvent
  (Utilities|FlowControl|Delay 2.0)
  (Game|SpawnActorfromClass "/Game/Roberto/Enemy/Grount/BattleEndGrount.BattleEndGrount_C" (Variables|Default|GetStartPoint) "Undefined" 0 0)
  (CallFunction|ActivateThunders false)
  (Actor|DestroyActor))

(event Custom|SetUpEnd
  (Input|DisableInput (Game|GetPlayerCharacter 0) (Game|GetPlayerController 0))
  (Variables|Default|SetbattleEnd true)
  (Transformation|SetWorldTransform (Variables|Collision|GetCapsuleComponent) (Variables|Default|GetStartPoint) false false)
  (bind _returnvalue (Sequencer|Player|CreateLevelSequencePlayer "/Game/Roberto/Stage3/Cinematic/NewFolder/Battle3MasterMaster.Battle3MasterMaster"))
  (Sequencer|Player|Play _returnvalue :!class /Script/MovieScene.MovieSceneSequencePlayer)
  (Utilities|Time|SetTimerbyEvent (delegate Custom|AntennaEvent) 3.0))

(event EventBeginPlay
  (bind _returnvalue (Actor|GetActorOfClass "/Game/OuKanu/Character/BP_Player.BP_Player_C"))
  (Variables|Default|Settarget _returnvalue)
  (Variables|Default|Setseq_max (Math|Random|RandomIntegerinRange 3 6))
  (Variables|Default|SetStartPoint (Transformation|GetWorldTransform (Variables|Collision|GetCapsuleComponent))))

(event EventTick
  (params (DeltaSeconds :type Float%20%28single-precision%29))
  ;[1 1 1] UPDATE
  (if (not (Variables|Default|GetbattleEnd))
    (if (|Activity)
      (if (Variables|Default|GetCatchPlayerAction)
        (CallFunction|SetPlayerPos)
        (if (not (Variables|Default|GetInAction))
          (CallFunction|ThrowPlayer DeltaSeconds))
        (else
          (Utilities|AttackCool DeltaSeconds)))
      (elif (Variables|Default|GetInAction)
        (CallFunction|SetPlayerPos)))))

(event Custom|PhysicalAttack
  (params (p :type Actor%20Object%20Reference))
  (bind _target (Variables|Default|Gettarget))
  ;[1 1 1] Physic Attack
  (bind _asbp_player (Utilities|Casting|CastToBP_Player p))
  (Utilities|IsValid _asbp_player
    (:Is%20Valid
      (Class|BPICharacter|Hurt(Message) p 2e+01)
      (Audio|SpawnSoundatLocation "/Game/Roberto/AudioManager/Music/SFX_Cue/Player_Hurt.Player_Hurt" (Transformation|GetActorLocation _target) "0, 0, 0" 1.0 1.0 0.0 0 0)
      (Effects|SpawnEmitteratLocation "/Game/OuKanu/FX/FXVarietyPack/Particles/P_ky_hit1.P_ky_hit1" (Transformation|GetActorLocation p))
      (Utilities|FlowControl|Delay 1.5)
      (bind _asbp_player_2 (Utilities|Casting|CastToBP_Player _target))
      (bind _currenthealth (Default|GetHealth _asbp_player_2))
      (if (<= _currenthealth 0.0)
        (Utilities|FlowControl|Delay 1.5)
        (bind _returnvalue (Game|GetCurrentLevelName true))
        (Game|OpenLevel(byName) (Utilities|String|StringToName _returnvalue))))))

(event Custom|Attack
  ;[1 1 1] Attack
  (bind _newparam (CallFunction|IsLowDistance 1e+03))
  (if _newparam
    (CallFunction|LowDistanceAtk)
    (Variables|Default|SetSequence 0)
    (elif (< (Variables|Default|GetSequence) (Variables|Default|Getseq_max))
      (Variables|Default|SetSequence (+ (Variables|Default|GetSequence) 1))
      (|RockCo)
      (else
        (bind _output_get (Variables|Default|Setrest_Counter (+ (Variables|Default|Getrest_Counter) 1.0)))
        (if (>= _output_get (Variables|Default|GetrestTime))
          (Variables|Default|Setrest_Counter 0.0)
          (Variables|Default|SetSequence 0)
          (Variables|Default|Setseq_max (Math|Random|RandomIntegerinRange 3 6)))))))

(event Custom|ResetStatus
  (bind _capsulecomponent (Variables|Collision|GetCapsuleComponent))
  (Variables|Default|SetInAction false)
  (Variables|Default|SetCatchPlayerAction false)
  (Physics|SetSimulatePhysics _capsulecomponent false)
  (Class|PrimitiveComponent|SetConstraintMode _capsulecomponent "YZPlane")
  (Transformation|SetActorRotation (Game|Player|GetPlayerPawn 0))
  (Utilities|FlowControl|Delay 1.5)
  (Variables|Default|Setmoving false))

(event Custom|MoveToPawn
  (params (target :type Pawn%20Object%20Reference))
  ;[1 1 1] Movement
  (Variables|Default|Setmoving true)
  (AI|AIMoveTo (Variables|Character|GetCharacterMovement) target "0, 0, 0" 0 5e+01 false
    (:OnSuccess
      _)
    (:OnFail
      _))
  (Variables|Default|Setmoving false))

(event Custom|MoveToV3
  (params (NewParam :type Vector))
  ;[1 1 1] Movement
  (Variables|Default|Setmoving true)
  (AI|AIMoveTo (Variables|Character|GetCharacterMovement) 0 NewParam 0 5e+01 false
    (:OnSuccess
      _)
    (:OnFail
      _))
  (Variables|Default|Setmoving false))

(event Custom|LowDistanceAtk
  ;[1 1 1] LOWATTACK
  (Utilities|FlowControl|Sequence
    (:then_0
      (Variables|Default|Setcurrent_action (Math|Random|RandomIntegerinRange 0 5)))
    (:then_1
      (bind _current_action (Utilities|AttackIndexCheckMacro))
      (|RelativeAvtion _current_action))
    (:then_2
      (Animation|PlayAnimMontage (Variables|Default|Getmontage) 1.0 "None"))))

(event Custom|AttachPlayer
  (params (NewParam :type Actor%20Object%20Reference))
  ;[1 1 1] LockPlayerPos
  (bind _asbp_player (Utilities|Casting|CastToBP_Player NewParam))
  (Utilities|IsValid _asbp_player
    (:Is%20Valid
      (if (not (Variables|Default|Getmoving))
        (Variables|Default|SetCatchPlayerAction true)))))

(event Custom|SetRootLoc
  ;[1 1 1] Rot
  (Transformation|SetWorldLocation (Variables|Collision|GetCapsuleComponent) (Transformation|GetWorldLocation (Variables|Character|GetMesh)) false false))

(event Custom|Hurt
  ;[1 1 1] Hurt
  (switch int (Math|Random|RandomIntegerinRange 0 3)
    (:Default
      (Animation|PlayAnimMontage "/Game/Roberto/Enemy/Grount/Animations/montages/mutant_Rib_Hit_Montage.mutant_Rib_Hit_Montage" 1.0 "None" :!label _label))
    (:0
      (goto _label))
    (:1
      (Animation|PlayAnimMontage "/Game/Roberto/Enemy/Grount/Animations/montages/mutant_Big_Stomach_Hit_Montage.mutant_Big_Stomach_Hit_Montage" 1.0 "None"))
    (:2
      (Animation|PlayAnimMontage "/Game/Roberto/Enemy/Grount/Animations/montages/mutant_Impact_Montage.mutant_Impact_Montage" 1.0 "None"))
    (:3
      (Animation|PlayAnimMontage "/Game/Roberto/Enemy/Grount/Animations/montages/mutant_Impact_Montage.mutant_Impact_Montage" 1.0 "None"))))

(event Custom|HurtPlayer
  (bind _target (Variables|Default|Gettarget))
  ;[1 1 1] Physic Attack
  (Class|BPICharacter|Hurt(Message) _target 2e+01)
  (Audio|SpawnSoundatLocation "/Game/Roberto/AudioManager/Music/SFX_Cue/Player_Hurt.Player_Hurt" (Transformation|GetActorLocation _target) "0, 0, 0" 1.0 1.0 0.0 0 0)
  (Effects|SpawnEmitteratLocation "/Game/OuKanu/FX/FXVarietyPack/Particles/P_ky_hit1.P_ky_hit1" (Transformation|GetActorLocation))
  (Utilities|FlowControl|Delay 1.5)
  (bind _asbp_player (Utilities|Casting|CastToBP_Player _target))
  (bind _currenthealth (Default|GetHealth _asbp_player))
  (if (<= _currenthealth 0.0)
    (Utilities|FlowControl|Delay 1.5)
    (bind _returnvalue (Game|GetCurrentLevelName true))
    (Game|OpenLevel(byName) (Utilities|String|StringToName _returnvalue))))

(event OnComponentBeginOverlap(Box)
  (params (OverlappedComponent :type Primitive%20Component%20Object%20Reference) (OtherActor :type Actor%20Object%20Reference) (OtherComp :type Primitive%20Component%20Object%20Reference) (OtherBodyIndex :type Integer) (bFromSweep :type Boolean) (SweepResult :type Hit%20Result%20Structure%20%28by%20ref%29))
  ;[1 1 1] HandColliders
  (if (Variables|Default|GetIsPhysical)
    (CallFunction|PhysicalAttack OtherActor)
    (else
      (CallFunction|AttachPlayer OtherActor))))

(event OnComponentBeginOverlap(Box1)
  (params (OverlappedComponent :type Primitive%20Component%20Object%20Reference) (OtherActor :type Actor%20Object%20Reference) (OtherComp :type Primitive%20Component%20Object%20Reference) (OtherBodyIndex :type Integer) (bFromSweep :type Boolean) (SweepResult :type Hit%20Result%20Structure%20%28by%20ref%29))
  ;[1 1 1] HandColliders
  (if (Variables|Default|GetIsPhysical)
    (CallFunction|PhysicalAttack OtherActor)
    (else
      (CallFunction|AttachPlayer OtherActor))))

(event OnComponentBeginOverlap(Box2)
  (params (OverlappedComponent :type Primitive%20Component%20Object%20Reference) (OtherActor :type Actor%20Object%20Reference) (OtherComp :type Primitive%20Component%20Object%20Reference) (OtherBodyIndex :type Integer) (bFromSweep :type Boolean) (SweepResult :type Hit%20Result%20Structure%20%28by%20ref%29))
  ;[1 1 1] FootColliders
  (CallFunction|PhysicalAttack OtherActor))

(event OnComponentBeginOverlap(Box3)
  (params (OverlappedComponent :type Primitive%20Component%20Object%20Reference) (OtherActor :type Actor%20Object%20Reference) (OtherComp :type Primitive%20Component%20Object%20Reference) (OtherBodyIndex :type Integer) (bFromSweep :type Boolean) (SweepResult :type Hit%20Result%20Structure%20%28by%20ref%29))
  ;[1 1 1] FootColliders
  (CallFunction|PhysicalAttack OtherActor))

(event Custom|ActivateBoth
  (params (NewParam :type Boolean))
  (bind _capsulecomponent (Variables|Collision|GetCapsuleComponent))
  ;[1 1 1] Hands
  (Utilities|FlowControl|Sequence
    (:then_0
      (Variables|Default|SetIsPhysical false))
    (:then_1
      (|ColliderOpen NewParam NewParam))
    (:then_2
      (if (not NewParam)
        (Physics|SetSimulatePhysics _capsulecomponent false)
        (Class|PrimitiveComponent|SetConstraintMode _capsulecomponent "Default")))))

(event Custom|ActivateFoot
  (params (NewParam :type Boolean))
  (bind _capsulecomponent (Variables|Collision|GetCapsuleComponent))
  ;[1 1 1] FootColliders
  (Utilities|FlowControl|Sequence
    (:then_0
      (bind _output_get (Variables|/Script/Engine.PrimitiveComponent|SetbGenerateOverlapEvents (Variables|Default|GetBox2) NewParam))
      (Variables|/Script/Engine.PrimitiveComponent|SetbGenerateOverlapEvents (Variables|Default|GetBox3) _output_get))
    (:then_1
      (if (not NewParam)
        (Physics|SetSimulatePhysics _capsulecomponent false)
        (Class|PrimitiveComponent|SetConstraintMode _capsulecomponent "Default")))))

(event Custom|ActivateThrowing
  (params (NewParam :type Boolean))
  (bind _capsulecomponent (Variables|Collision|GetCapsuleComponent))
  ;[1 1 1] ThrowActionCollider
  (Utilities|FlowControl|Sequence
    (:then_0
      (Variables|Default|SetIsPhysical false)
      (Physics|SetSimulatePhysics _capsulecomponent false)
      (Class|PrimitiveComponent|SetConstraintMode _capsulecomponent "Default"))
    (:then_1
      (|OpneClose NewParam NewParam))))

(fn ConstructionScript)

(fn TakeDamage
  (if (not (Variables|Default|GetisDeath))
    (bind _output_get (Variables|Default|SetHp (- (Variables|Default|GetHp) 1)))
    (if (<= _output_get 0)
      (if (not (Variables|Default|GetbattleEnd))
        (CallFunction|Hurt))
      (else
        (CallFunction|Hurt)))))

(fn EndBattle
  (Variables|Default|SetInBattle false)
  (Variables|Default|SetbattleEnd true)
  (bind _asgrount_animator (Utilities|Casting|CastToGrountAnimator (Components|SkeletalMesh|GetAnimInstance (Variables|Character|GetMesh))))
  (Variables|/Game/Roberto/Enemy/Grount/GrountAnimator.GrountAnimator_C|SetisDeath _asgrount_animator true))

(fn GenerateStone
  (bind _returnvalue (Game|SpawnActorfromClass "/Game/Roberto/Enemy/Grount/Rock/BossRockBP.BossRockBP_C" (Math|Transform|MakeTransform "0, 0, 0" "0, 0, 0" "1,1,1") "Undefined" 0 0))
  (bind _output_get (Variables|Default|SetCurrentStone1 _returnvalue))
  (if (Variables|Default|GetisLeft)
    (Transformation|AttachComponentToComponent _output_get (Variables|Default|GetLeftHandSocket) "None" "KeepRelative" "KeepRelative" "KeepRelative" true)
    (else
      (Transformation|AttachComponentToComponent _output_get (Variables|Default|GetRighHandSocket) "None" "KeepRelative" "KeepRelative" "KeepRelative" true)))
  (Default|INITIALIZE (Variables|Default|GetCurrentStone1)))

(fn ThrowStone
  (bind _currentstone1 (Variables|Default|GetCurrentStone1))
  (Transformation|AttachComponentToComponent _currentstone1 0 "None" "KeepRelative" "KeepRelative" "KeepRelative" true)
  (Physics|SetSimulatePhysics (Variables|/Game/Roberto/Enemy/Grount/Rock/BossRockBP.BossRockBP_C|GetModel _currentstone1) true)
  (CallFunction|CalculateRockSpeed)
  (Default|MoveRock (Variables|Default|GetCurrentStone1) (Transformation|GetActorLocation (Game|Player|GetPlayerPawn 0)) (Variables|Default|Getrockspeed)))

(fn LockPlayer
  (bind _target (Variables|Default|Gettarget))
  (Utilities|IsValid _target
    (:Is%20Valid
      (Transformation|SetWorldRotation (Variables|Collision|GetCapsuleComponent) (Math|Rotator|MakeRotator 0.0 0.0 (.yaw (Math|Rotator|FindLookatRotation (Transformation|GetActorLocation) (Transformation|GetActorLocation _target)))) false false))))

(fn Cooldown
  (params (time :type Float%20%28single-precision%29))
  (bind _output_get (Variables|Default|SetatkCounter (+ (Variables|Default|GetatkCounter) time)))
  (if (>= _output_get (Variables|Default|GetattackTime))
    (Variables|Default|SetatkCounter 0.0)
    (Variables|Default|Setattaking true)))

(fn IsLowDistance
  (params (distanceToCheck :type Float%20%28single-precision%29))
  (return (<= (Transformation|GetDistanceTo (Game|Player|GetPlayerPawn 0)) distanceToCheck)))

(fn SetPlayerPos
  (bind _returnvalue (Game|Player|GetPlayerPawn 0))
  (if (not (Variables|Default|GetisLeft))
    (Transformation|SetActorLocation _returnvalue (+ (Transformation|GetWorldLocation (Variables|Default|GetRighHandSocket)) (Variables|Default|GethandZOffset)) false false)
    (else
      (Transformation|SetActorLocation _returnvalue (+ (Transformation|GetWorldLocation (Variables|Default|GetLeftHandSocket)) (Variables|Default|GethandZOffset)) false false))))

(fn ThrowPlayer
  (params (Delta :type Float%20%28single-precision%29))
  (bind _output_get (Variables|Default|SettrowCounter (+ (Variables|Default|GettrowCounter) Delta)))
  (if (> _output_get 1.0)
    (Variables|Default|SetatkCounter 0.0)
    (Variables|Default|SetCatchPlayerAction false)
    (Variables|Default|SetInAction true)
    (Variables|Default|Setmoving true)
    (if (Variables|Default|GetisLeft)
      (Animation|PlayAnimMontage "/Game/Roberto/Enemy/Grount/Animations/montages/ComboLeft.ComboLeft" 1.0 "None")
      (else
        (Animation|PlayAnimMontage "/Game/Roberto/Enemy/Grount/Animations/montages/ComboRIght.ComboRIght" 1.0 "None")))))

(fn CalculateRockSpeed
  (Utilities|FlowControl|Sequence
    (:then_0
      (LocalVariables|Setamount (Transformation|GetDistanceTo (Game|Player|GetPlayerPawn 0) self))
      (bind _output_get (Variables|Default|Setrockspeed (* (LocalVariables|Getamount) 0.001 0.5)))
      (if (<= _output_get 0.7)
        (Variables|Default|Setrockspeed 1.0)))
    (:then_2
      (return))))

(fn ActivateThunders
  (params (V/f :type Boolean))
  (for _array_element (Variables|Default|GetThunders)
    (Rendering|SetActorHiddenInGame _array_element V/f)))

(event Custom|MoveUP
  (bind _capsulecomponent (Variables|Collision|GetCapsuleComponent))
  (bind _capsulecomponent_2 (Variables|Collision|GetCapsuleComponent))
  (Physics|SetSimulatePhysics _capsulecomponent_2 true)
  (Class|PrimitiveComponent|SetConstraintMode _capsulecomponent_2 "CustomPlane")
  (Physics|AddImpulse _capsulecomponent (* (Math|Vector|GetForwardVector _capsulecomponent) 3.5e+02) "None" true))