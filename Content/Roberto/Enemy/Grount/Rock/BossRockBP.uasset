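; BossRockBP is a rock actor, filed under the Grount enemy, that randomizes its shape when initialized.
; Its INITIALIZE event calls SetSize, which gives the Model component an independent random scale on each axis, then SetLocation.
; SetLocation resets the actor's relative location to the origin, without sweep or teleport.
; BeginPlay, Tick and the construction script are empty, so nothing happens until INITIALIZE is called.
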(event Custom|INITIALIZE
  (CallFunction|SetSize)
  (CallFunction|SetLocation))

(event EventBeginPlay)

(event Collision|EventActorBeginOverlap
  (params (OtherActor :type Actor%20Object%20Reference)))

(event EventTick
  (params (DeltaSeconds :type Float%20%28single-precision%29)))

(fn ConstructionScript)

(fn SetSize
  (Variables|Default|Setx (Math|Random|RandomFloatinRange 0.5 4.0))
  (Variables|Default|Sety (Math|Random|RandomFloatinRange 0.5 4.0))
  (Variables|Default|Setz (Math|Random|RandomFloatinRange 0.5 4.0))
  (Transformation|SetRelativeScale3D (Variables|Default|GetModel) (Math|Vector|MakeVector (Variables|Default|Getx) (Variables|Default|Gety) (Variables|Default|Getz))))

(fn SetLocation
  (Transformation|SetActorRelativeLocation "0, 0, 0"))