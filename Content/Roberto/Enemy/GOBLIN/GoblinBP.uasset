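; Goblin boss character that faces the player and lobs grenades during its battle, ending Stage 2 on death.
; While stationary in battle, Tick runs an attack timer that picks random throw montages; ThrowBomb spawns BP_Granade with force scaled by player distance.
; Exposed events handle AI movement, reaction montages and attack toggling, while Hurt forwards damage to GoblinBattleController.
; Die stops attacks, plays the death animation and end cutscene, then loads the Stage 3 transition.
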(event Custom|SetTargetDestination
  (params (pos :type Actor%20Object%20Reference))
  ;[1 1 1] MOVEMENT
  (Variables|Default|Setmoving true)
  (AI|AIMoveTo (Pawn|GetControlledPawn (Variables|Default|GetAI)) "0, 0, 0" pos 1e+02 false
    (:OnSuccess
      _)
    (:OnFail
      _))
  (Variables|Default|Setmoving false))

(event Custom|SetDestination
  (params (pos :type Vector))
  ;[1 1 1] MOVEMENT
  (Variables|Default|Setmoving true)
  (AI|AIMoveTo (Pawn|GetControlledPawn (Variables|Default|GetAI)) pos 0 1e+02 false
    (:OnSuccess
      _)
    (:OnFail
      _))
  (Variables|Default|Setmoving false))

(event Custom|Die
  (CallFunction|BlockAttack)
  (Input|DisableInput (Game|GetPlayerCharacter 0) (Game|GetPlayerController 0))
  (bind _asgoblin_boss_animator (Utilities|Casting|CastToGoblinBossAnimator (Components|SkeletalMesh|GetAnimInstance (Variables|Character|GetMesh))))
  (Default|Death _asgoblin_boss_animator)
  (Utilities|FlowControl|Delay 3.0)
  (Rendering|SetVisibility (Variables|Character|GetMesh) false false)
  (CallFunction|EndGameCutScene))

(event Custom|BlockAttack
  (Variables|Default|SetatkTime 0.0)
  (Variables|Default|SetInBattle false))

(event Custom|ActivateAttackLoop
  (CallFunction|RotateinPlayerDir)
  (Variables|Default|SetatkTime 3.0)
  (Variables|Default|SetInBattle true))

(event Custom|EndGameCutScene
  ;[1 1 1] EndBattleCutScene
  (Input|DisableInput (Game|GetPlayerCharacter 0) (Game|GetPlayerController 0))
  (bind _returnvalue (Actor|GetActorOfClass "/Game/OuKanu/Character/BP_Player.BP_Player_C"))
  (Rendering|SetActorHiddenInGame _returnvalue false)
  (bind _returnvalue_2 (Sequencer|Player|CreateLevelSequencePlayer "/Game/Roberto/GoblinEndSequence/GoblinEndSequenceMaster.GoblinEndSequenceMaster"))
  (Sequencer|Player|Play _returnvalue_2 :!class /Script/MovieScene.MovieSceneSequencePlayer)
  (Utilities|FlowControl|Delay 3e+01)
  (Game|OpenLevel(byName) "LoadingFromStage2ToStage3"))

(event EventBeginPlay
  ;[1 1 1] START
  (Variables|Default|SetAI (AI|GetAIController self)))

(event EventHurt
  (params (Damage :type Float%20%28single-precision%29))
  ;[1 1 1] HURT
  (if (Variables|Default|GetInBattle)
    (bind _returnvalue (Actor|GetActorOfClass "/Game/Roberto/Enemy/GOBLIN/GoblinBattleController.GoblinBattleController_C"))
    (Utilities|IsValid _returnvalue
      (:Is%20Valid
        (Default|OnTakingDamage _returnvalue)))))

(event EventTick
  (params (DeltaSeconds :type Float%20%28single-precision%29))
  ;[1 1 1] UPDATE
  (if (not (Variables|Default|Getmoving))
    (CallFunction|RotateinPlayerDir)
    (if (Variables|Default|GetInBattle)
      (CallFunction|Combat DeltaSeconds))))

(event Custom|ThrowRightDown
  (Animation|PlayAnimMontage "/Game/Roberto/Enemy/GOBLIN/NewModel/Montages/Throw__1__Montage.Throw__1__Montage" 1.0 "None"))

(event Custom|ThrowLeft
  (Animation|PlayAnimMontage "/Game/Roberto/Enemy/GOBLIN/NewModel/Montages/Grenade_Throw__1__Montage.Grenade_Throw__1__Montage" 2.0 "None"))

(event Custom|Laugh
  (Animation|PlayAnimMontage "/Game/Roberto/Enemy/GOBLIN/CUTSCENE/Laughing__1__Montage.Laughing__1__Montage" 1.0 "None"))

(event Custom|ThrowRight
  (Animation|PlayAnimMontage "/Game/Roberto/Enemy/GOBLIN/NewModel/Montages/Grenade_Throw_Montage.Grenade_Throw_Montage" 2.0 "None"))

(event Custom|Angry
  (Animation|PlayAnimMontage "/Game/Roberto/Enemy/GOBLIN/NewModel/Montages/Angry_Anim_mixamo_com_Montage.Angry_Anim_mixamo_com_Montage" 2.7 "None"))

(event Custom|ThrowLeftDown
  (Animation|PlayAnimMontage "/Game/Roberto/Enemy/GOBLIN/NewModel/Montages/Throw_Montage.Throw_Montage" 1.0 "None"))

(event Custom|Yeling
  (Animation|PlayAnimMontage "/Game/Roberto/Enemy/GOBLIN/NewModel/Montages/Yelling_Anim_mixamo_com_Montage.Yelling_Anim_mixamo_com_Montage" 1.5 "None"))

(event Custom|Scream
  (Animation|PlayAnimMontage "/Game/Roberto/Enemy/GOBLIN/NewModel/Montages/Zombie_Scream_Anim_mixamo_com_Montage.Zombie_Scream_Anim_mixamo_com_Montage" 1.0 "None"))

(event Custom|HurtAnimation
  (Animation|PlayAnimMontage "/Game/Roberto/Enemy/GOBLIN/NewModel/Montages/Injured_Hurting_Idle_Montage.Injured_Hurting_Idle_Montage" 2.0 "None"))

(event Custom|Combat
  (params (delta :type Float%20%28single-precision%29))
  ;[1 1 1] Phase1
  (bind _output_get (Variables|Default|SetatkTime (+ delta (Variables|Default|GetatkTime))))
  (if (>= _output_get (Variables|Default|GetatkDelay))
    (Variables|Default|SetatkTime 0.0)
    (CallFunction|RandAttack)))

(fn ConstructionScript)

(fn UseJump)

(fn ThrowBomb
  (if true
    (CallFunction|CalculateDistance)
    (else
      (Variables|Default|Setdistance 5e+03)))
  (CallFunction|SpawnBomb))

(fn SpawnBomb
  (if (Variables|Default|GetInBattle)
    (bind _output_get (LocalVariables|SetDestination (* (Transformation|GetActorForwardVector) 1e+02)))
    (bind _returnvalue (Game|SpawnActorfromClass "/Game/Roberto/Enemy/GOBLIN/Granade/BP_Granade.BP_Granade_C" (Transformation|GetWorldTransform (Variables|Default|GetArrow1)) "Undefined" 0 0))
    (bind _output_get_2 (LocalVariables|SetnewBomb _returnvalue))
    (Utilities|IsValid _output_get_2
      (:Is%20Valid
        (Default|Throw _output_get_2 _output_get (* (Variables|Default|GetForceMultipler) (Variables|Default|Getdistance)) self)))))

(fn CalculateDistance
  (Variables|Default|Setdistance (Transformation|GetDistanceTo self (Variables|Default|GetPlayer))))

(fn RotateinPlayerDir
  (bind _playerexist (CallFunction|LookforPlayer))
  (if _playerexist
    (Transformation|SetActorRotation (Math|Rotator|MakeRotator 0.0 0.0 (.yaw (Math|Rotator|FindLookatRotation (Transformation|GetActorLocation) (Transformation|GetActorLocation (Variables|Default|GetPlayer)))))))
  (return _playerexist))

(fn LookforPlayer
  (Utilities|IsValid (Variables|Default|GetPlayer)
    (:Is%20Valid
      (LocalVariables|SetIsValid true :!label _label))
    (:Is%20Not%20Valid
      (bind _returnvalue (Actor|GetActorOfClass "/Game/OuKanu/Character/BP_Player.BP_Player_C"))
      (bind _output_get (Variables|Default|SetPlayer _returnvalue))
      (Utilities|IsValid _output_get
        (:Is%20Valid
          (goto _label))
        (:Is%20Not%20Valid
          (LocalVariables|SetIsValid false)))))
  (return (LocalVariables|GetIsValid)))

(fn RandAttack
  (switch int (Math|Random|RandomIntegerinRange 1 4)
    (:0
      (CallFunction|ThrowLeft))
    (:1
      (CallFunction|ThrowRight))
    (:2
      (CallFunction|ThrowLeftDown))
    (:3
      (CallFunction|ThrowRightDown))))

(fn MakeVisible
  (params (VF :type Boolean))
  (Rendering|SetVisibility (Variables|Character|GetMesh) VF false))

(fn GetIsDead
  (return false))

(fn IsHoldingBottle
  (return false))