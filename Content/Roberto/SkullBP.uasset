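; Skull actor that can spin, slide along a path and explode in a puff, driven by Spin, reverse and Explode events.
; Spin and reverse play a timeline forward or backward, offsetting X and Y from the start position while Tick adds yaw until it finishes.
; Explode plays poof sound and hit particles at a valid OtherSkulk, then after a short delay at its own location, with destroy calls after each.
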(event Custom|Spin
  (bind _startpos (Variables|Default|GetstartPos))
  (Variables|Default|Setrotating true)
  (bind (_direction _outy _outx) (Timeline|movetimeline Play)
    (:Update
      (Transformation|SetWorldLocation (Variables|Default|GetDefaultSceneRoot) (Math|Vector|MakeVector (+ (.x _startpos) _outx) (+ (.y _startpos) _outy) (.z _startpos)) false false))
    (:Finished
      (Variables|Default|Setrotating false))))

(event Custom|reverse
  (bind _startpos (Variables|Default|GetstartPos))
  (Variables|Default|Setrotating true)
  (bind (_direction _outy _outx) (Timeline|movetimeline Reverse)
    (:Update
      (Transformation|SetWorldLocation (Variables|Default|GetDefaultSceneRoot) (Math|Vector|MakeVector (+ (.x _startpos) _outx) (+ (.y _startpos) _outy) (.z _startpos)) false false))
    (:Finished
      (Variables|Default|Setrotating false))))

(event Custom|Explode
  (bind _otherskulk (Variables|Default|GetotherSkulk))
  (bind _defaultsceneroot (Variables|Default|GetDefaultSceneRoot))
  (bind _returnvalue (Transformation|GetActorLocation _otherskulk))
  (bind _returnvalue_2 (Transformation|GetWorldLocation _defaultsceneroot))
  (Utilities|IsValid _otherskulk
    (:Is%20Valid
      (Audio|PlaySoundatLocation "/Game/Roberto/Poof.Poof" _returnvalue "0, 0, 0" 1.0 1.0 0.0 0 0 0)
      (Effects|SpawnEmitteratLocation "/Game/OuKanu/FX/FXVarietyPack/Particles/P_ky_hit2.P_ky_hit2" _returnvalue)
      (Actor|DestroyActor))
    (:Is%20Not%20Valid
      _))
  (Utilities|FlowControl|Delay 0.2)
  (Audio|PlaySoundatLocation "/Game/Roberto/Poof.Poof" _returnvalue_2 "0, 0, 0" 1.0 1.0 0.0 0 0 0)
  (Effects|SpawnEmitteratLocation "/Game/OuKanu/FX/FXVarietyPack/Particles/P_ky_hit2.P_ky_hit2" _returnvalue_2)
  (Actor|DestroyActor))

(event EventBeginPlay
  (Variables|Default|SetstartPos (Transformation|GetWorldLocation (Variables|Default|GetDefaultSceneRoot))))

(event EventTick
  (params (DeltaSeconds :type Float%20%28single-precision%29))
  (bind _defaultsceneroot (Variables|Default|GetDefaultSceneRoot))
  (bind _returnvalue (Transformation|GetWorldRotation _defaultsceneroot))
  (if (Variables|Default|Getrotating)
    (Transformation|SetWorldRotation (Variables|Default|GetDefaultSceneRoot) (Math|Rotator|MakeRotator (.roll _returnvalue) (.pitch _returnvalue) (+ (.yaw _returnvalue) 5.0)) false false)))

(fn ConstructionScript)