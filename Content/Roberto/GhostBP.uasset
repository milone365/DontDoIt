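; GhostBP is a ghost hazard actor that hurts BP_Player on overlap.
; BeginPlay randomly picks one of two sounds and applies the same laser material in either case.
; MoveSpider plays the sound and uses a timeline to shift the root along negative X, then bursts and destroys the actor after a delay.
; Player overlap calls HurtMessage once, spawns the hit emitter on the player and destroys the ghost.
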(event OnComponentBeginOverlap(Box)
  (params (OverlappedComponent :type Primitive%20Component%20Object%20Reference) (OtherActor :type Actor%20Object%20Reference) (OtherComp :type Primitive%20Component%20Object%20Reference) (OtherBodyIndex :type Integer) (bFromSweep :type Boolean) (SweepResult :type Hit%20Result%20Structure%20%28by%20ref%29))
  (bind _asbp_player (Utilities|Casting|CastToBP_Player OtherActor))
  (Utilities|IsValid _asbp_player
    (:Is%20Valid
      (if (not (Variables|Default|Getd))
        (Variables|Default|Setd true)
        (Class|BPICharacter|Hurt(Message) _asbp_player 6e+01)
        (Effects|SpawnEmitteratLocation "/Game/OuKanu/FX/FXVarietyPack/Particles/P_ky_hit1.P_ky_hit1" (Transformation|GetWorldLocation (Variables|/Script/Engine.Character|GetMesh _asbp_player)))
        (Actor|DestroyActor)))))

(event Custom|MoveSpider
  (bind _defaultsceneroot (Variables|Default|GetDefaultSceneRoot))
  (bind _returnvalue (Transformation|GetWorldLocation _defaultsceneroot))
  (Audio|Components|Audio|Play (Variables|Default|GetAudio) 0.0)
  (bind _returnamount (Timeline|Timeline_0 Play)
    (:Update
      (Components|MoveComponentTo (Variables|Default|GetDefaultSceneRoot) (Math|Vector|MakeVector (- (.x _returnvalue) _returnamount) (.y _returnvalue) (.z _returnvalue)) (Transformation|GetWorldRotation _defaultsceneroot) false false 0.2 false))
    (:Finished
      (Utilities|FlowControl|Delay 2.0)
      (Effects|SpawnEmitteratLocation "/Game/OuKanu/FX/FXVarietyPack/Particles/P_ky_hit1.P_ky_hit1" (Transformation|GetWorldLocation (Variables|Default|GetStaticMesh)))
      (Actor|DestroyActor))))

(event EventBeginPlay
  (if (> (Math|Random|RandomIntegerinRange 1 10) 5)
    (Audio|Components|Audio|SetSound (Variables|Default|GetAudio) "/Game/Roberto/Stage3/JumpScare/_Indonesia._Indonesia")
    (Rendering|Material|SetMaterial (Variables|Default|GetStaticMesh) 0 "/Game/Roberto/LASER/Ma/LaserMaterial_Inst.LaserMaterial_Inst")
    (else
      (Audio|Components|Audio|SetSound (Variables|Default|GetAudio) "/Game/Roberto/Stage3/JumpScare/Ghost1.Ghost1")
      (Rendering|Material|SetMaterial (Variables|Default|GetStaticMesh) 0 "/Game/Roberto/LASER/Ma/LaserMaterial_Inst.LaserMaterial_Inst"))))

(fn ConstructionScript)