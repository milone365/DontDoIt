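; PulledFlushBP is a hazard volume that repeatedly hurts the player while they stay inside its box.
; Box overlaps cache the BP_Player and toggle a flag, letting Tick count down a damage interval that resets outside the area.
; Each hit applies fixed damage and attaches a particle effect to the player's mesh, removed after a delay if they survive.
; At zero health, it reloads the current level after a short delay.
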(event OnComponentBeginOverlap(Box)
  (params (OverlappedComponent :type Primitive%20Component%20Object%20Reference) (OtherActor :type Actor%20Object%20Reference) (OtherComp :type Primitive%20Component%20Object%20Reference) (OtherBodyIndex :type Integer) (bFromSweep :type Boolean) (SweepResult :type Hit%20Result%20Structure%20%28by%20ref%29))
  (bind _asbp_player (Utilities|Casting|CastToBP_Player OtherActor))
  (Utilities|IsValid _asbp_player
    (:Is%20Valid
      (Variables|Default|SetPlayer _asbp_player)
      (Variables|Default|SetInArea true))))

(event OnComponentEndOverlap(Box)
  (params (OverlappedComponent :type Primitive%20Component%20Object%20Reference) (OtherActor :type Actor%20Object%20Reference) (OtherComp :type Primitive%20Component%20Object%20Reference) (OtherBodyIndex :type Integer))
  (bind _asbp_player (Utilities|Casting|CastToBP_Player OtherActor))
  (Utilities|IsValid _asbp_player
    (:Is%20Valid
      (Variables|Default|SetInArea false))))

(event EventBeginPlay)

(event Collision|EventActorBeginOverlap
  (params (OtherActor :type Actor%20Object%20Reference)))

(event EventTick
  (params (DeltaSeconds :type Float%20%28single-precision%29))
  (bind _player (Variables|Default|GetPlayer))
  (if (Variables|Default|GetInArea)
    (bind _output_get (Variables|Default|SetTimeCounter (- (Variables|Default|GetTimeCounter) DeltaSeconds)))
    (if (<= _output_get 0.0)
      (Variables|Default|SetTimeCounter (Variables|Default|GetdamageTime))
      (Class|BPICharacter|Hurt(Message) _player 2e+01)
      (bind _returnvalue (Effects|SpawnEmitterAttached "/Game/Chokxunxiong/ARt/Test/Test/Style/smoke1/sub.sub" (Variables|/Script/Engine.Character|GetMesh _player) "None" (Variables|Default|GetPos)))
      (Variables|Default|SetlocalSmoke _returnvalue)
      (bind _currenthealth (Default|GetHealth _player))
      (if (<= _currenthealth 0.0)
        (if (not (Variables|Default|GetboolIsDeath))
          (Variables|Default|SetboolIsDeath true)
          (Utilities|FlowControl|Delay 1.0)
          (bind _returnvalue_2 (Game|GetCurrentLevelName true))
          (Game|OpenLevel(byName) (Utilities|String|StringToName _returnvalue_2)))
        (else
          (Utilities|FlowControl|Delay 3.0)
          (Components|DestroyComponent (Variables|Default|GetlocalSmoke)))))
    (else
      (Variables|Default|SetTimeCounter (Variables|Default|GetdamageTime)))))

(fn ConstructionScript)