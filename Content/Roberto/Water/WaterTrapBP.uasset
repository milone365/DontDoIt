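; Rising water trap actor that scales a cube upward and damages a player inside it.
; After a start delay it activates, growing Z scale each Tick to a maximum, or shrinking toward start size when inactive.
; While rising, overlap tracking drives timed damage, reloading the level on death.
; HeightCheck, uncalled here, reloads the level if Top passes Roof with the player inside.
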(event OnComponentBeginOverlap(Cube)
  (params (OverlappedComponent :type Primitive%20Component%20Object%20Reference) (OtherActor :type Actor%20Object%20Reference) (OtherComp :type Primitive%20Component%20Object%20Reference) (OtherBodyIndex :type Integer) (bFromSweep :type Boolean) (SweepResult :type Hit%20Result%20Structure%20%28by%20ref%29))
  ;[1 1 1] OVERLAP_START_END
  (bind _asbp_player (Utilities|Casting|CastToBP_Player OtherActor))
  (Utilities|IsValid _asbp_player
    (:Is%20Valid
      (Variables|Default|SetPlayer _asbp_player)
      (Variables|Default|SetplayerInZone true))))

(event OnComponentEndOverlap(Cube)
  (params (OverlappedComponent :type Primitive%20Component%20Object%20Reference) (OtherActor :type Actor%20Object%20Reference) (OtherComp :type Primitive%20Component%20Object%20Reference) (OtherBodyIndex :type Integer))
  ;[1 1 1] OVERLAP_START_END
  (bind _asbp_player (Utilities|Casting|CastToBP_Player OtherActor))
  (Utilities|IsValid _asbp_player
    (:Is%20Valid
      (Variables|Default|SetplayerInZone false))))

(event Custom|LevelDown
  (bind _cube (Variables|Default|GetCube))
  (bind _speed (Variables|Default|GetSpeed))
  (bind _returnvalue (Transformation|GetWorldScale _cube))
  (bind _returnvalue_2 (- (.z _returnvalue) _speed))
  ;[1 1 1] Deactivation
  (Transformation|SetWorldScale3D _cube (Math|Vector|MakeVector (.x _returnvalue) (.y _returnvalue) _returnvalue_2))
  (Variables|Default|SetCurentSize _returnvalue_2))

(event Custom|ActivateTrap
  (Variables|Default|SettrapActive true))

(event Custom|LevelUp
  (bind _cube (Variables|Default|GetCube))
  (bind _speed (Variables|Default|GetSpeed))
  (bind _speedmultipler (Variables|Default|GetSpeedMultipler))
  (bind _returnvalue (Transformation|GetWorldScale _cube))
  (bind _returnvalue_2 (* _speed _speedmultipler))
  (bind _returnvalue_3 (+ (.z _returnvalue) _returnvalue_2))
  ;[1 1 1] ACTIVATION
  (Transformation|SetWorldScale3D _cube (Math|Vector|MakeVector (.x _returnvalue) (.y _returnvalue) _returnvalue_3))
  (Variables|Default|SetCurentSize _returnvalue_3))

(event EventBeginPlay
  ;[1 1 1] START
  (bind _output_get (Variables|Default|SetStartSize (.x (Variables|/Script/Engine.SceneComponent|GetRelativeScale3D (Variables|Default|GetCube)))))
  (Variables|Default|SetCurentSize _output_get)
  (Utilities|FlowControl|Delay (Variables|Default|GetactivationCooldown))
  (CallFunction|ActivateTrap))

(event EventTick
  (params (DeltaSeconds :type Float%20%28single-precision%29))
  ;[1 1 1] UPDATE
  (if (Variables|Default|GettrapActive)
    (if (< (Variables|Default|GetCurentSize) (Variables|Default|GetMaxSize))
      (CallFunction|LevelUp)
      (Utilities|HurtMacro DeltaSeconds))
    (elif (> (Variables|Default|GetCurentSize) (Variables|Default|GetStartSize))
      (CallFunction|LevelDown))))

(fn ConstructionScript)

(fn Activate
  (Variables|Default|SettrapActive true))

(fn HeightCheck
  (bind _roof (Variables|Default|GetRoof))
  (if (Variables|Default|GetplayerInZone)
    (Utilities|IsValid _roof
      (:Is%20Valid
        (if (> (.z (Transformation|GetWorldLocation (Variables|Default|GetTop))) (.z (Transformation|GetWorldLocation (Variables|/Script/Engine.Actor|GetRootComponent _roof))))
          (bind _returnvalue (Game|GetCurrentLevelName true))
          (Game|OpenLevel(byName) (Utilities|String|StringToName _returnvalue)))))))