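; Carryable flag actor that shows one of several national flags, picking its child actor class from Nation at BeginPlay.
; Overlapping its box attaches it to a player without a load, and Tick snaps it to their right hand.
; Pressing Y or gamepad top face button drops it at its original height with a fixed rotation and frees the player.
; A one-shot Deactivation event detaches and destroys it after a short delay.
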(event OnComponentBeginOverlap(Box)
  (params (OverlappedComponent :type Primitive%20Component%20Object%20Reference) (OtherActor :type Actor%20Object%20Reference) (OtherComp :type Primitive%20Component%20Object%20Reference) (OtherBodyIndex :type Integer) (bFromSweep :type Boolean) (SweepResult :type Hit%20Result%20Structure%20%28by%20ref%29))
  ;[1 1 1] TRIGGER
  (bind _asbp_player (Utilities|Casting|CastToBP_Player OtherActor))
  (bind _output_get (Variables|Default|SetPlayerChar _asbp_player))
  (Utilities|IsValid _output_get
    (:Is%20Valid
      (if (not (Variables|/Game/OuKanu/Character/BP_Character.BP_Character_C|GetHaveWeight (Variables|Default|GetPlayerChar)))
        (Variables|/Game/OuKanu/Character/BP_Character.BP_Character_C|SetHaveWeight (Variables|Default|GetPlayerChar) true)
        (Variables|Default|Setattached true)
        (Default|SetText (Variables|Default|Getwiget) "Drop flag with Y")))))

(event Custom|SetHandLocation
  (bind _playerchar (Variables|Default|GetPlayerChar))
  (bind _defaultsceneroot (Variables|Default|GetDefaultSceneRoot))
  (bind _righthandlocation (Variables|/Game/OuKanu/Character/BP_Character.BP_Character_C|GetRightHandLocation _playerchar))
  ;[1 1 1] Set Position and Rotation
  (Transformation|SetWorldLocation _defaultsceneroot (Transformation|GetSocketLocation _righthandlocation "None") false false)
  (Transformation|SetRelativeRotation _defaultsceneroot (Transformation|GetWorldRotation _righthandlocation) false false))

(event Custom|Deactivation
  ;[1 1 1] Deleteflag
  (if (not (Variables|Default|GetClosed))
    (Variables|Default|SetClosed true)
    (Variables|Default|Setattached false)
    (Utilities|FlowControl|Delay 0.25)
    (Actor|DestroyActor)))

(event EventTick
  (params (DeltaSeconds :type Float%20%28single-precision%29))
  (if (Variables|Default|Getattached)
    (CallFunction|SetHandLocation)
    (bind _v (CallFunction|GetInput))
    (if _v
      (Variables|Default|Setattached false)
      (Utilities|FlowControl|Delay 0.25)
      (Variables|/Game/OuKanu/Character/BP_Character.BP_Character_C|SetHaveWeight (Variables|Default|GetPlayerChar) false)
      (Default|SetText (Variables|Default|Getwiget))
      (CallFunction|Poseflag))))

(event EventBeginPlay
  (CallFunction|SetRelativeFlag)
  (bind _output_get (Variables|Default|SetstartPos (Transformation|GetWorldLocation (Variables|Default|GetDefaultSceneRoot))))
  (Variables|Default|SetHeight (.z _output_get)))

(fn ConstructionScript)

(fn SetRelativeFlag
  (Utilities|FlowControl|Sequence
    (:then_0
      (switch Utilities|FlowControl|Switch|SwitchonCounties (Variables|Default|GetNation)
        (:NewEnumerator0
          (LocalVariables|Setflag "/Game/Roberto/Geography/FlagsBP/Italy_FlagBP.Italy_FlagBP_C"))
        (:NewEnumerator1
          (LocalVariables|Setflag "/Game/Roberto/Geography/FlagsBP/Spain_blag_bp.Spain_blag_bp_C"))
        (:NewEnumerator2
          (LocalVariables|Setflag "/Game/Roberto/Geography/FlagsBP/Australia_flag_bp.Australia_flag_bp_C"))
        (:NewEnumerator3
          (LocalVariables|Setflag "/Game/Roberto/Geography/FlagsBP/Sweden_fagBP.Sweden_fagBP_C"))
        (:NewEnumerator4
          (LocalVariables|Setflag "/Game/Roberto/Geography/FlagsBP/Japan_FlagBp.Japan_FlagBp_C"))
        (:NewEnumerator5
          (LocalVariables|Setflag "/Game/Roberto/Geography/FlagsBP/Korea_Flag_bp.Korea_Flag_bp_C"))
        (:NewEnumerator6
          (LocalVariables|Setflag "/Game/Roberto/Geography/FlagsBP/China_Flag_Bp.China_Flag_Bp_C"))
        (:NewEnumerator7
          (LocalVariables|Setflag "/Game/Roberto/Geography/FlagsBP/Taiwan_flagBo.Taiwan_flagBo_C"))
        (:NewEnumerator8
          (LocalVariables|Setflag "/Game/Roberto/Geography/FlagsBP/FlagBP.FlagBP_C"))))
    (:then_1
      (ChildActorComponent|SetChildActorClass (Variables|Default|GetChildActor) (LocalVariables|Getflag)))))

(fn GetInput
  (Utilities|FlowControl|Sequence
    (:then_0
      (if (Game|Player|IsInputKeyDown (Game|GetPlayerController 0) "Gamepad_FaceButton_Top")
        (LocalVariables|SetNewLocalVar_0 true :!label _label)
        (elif (Game|Player|IsInputKeyDown (Game|GetPlayerController 0) "Y")
          (goto _label))))
    (:then_1
      (return (LocalVariables|GetNewLocalVar_0)))))

(fn Poseflag
  (bind _defaultsceneroot (Variables|Default|GetDefaultSceneRoot))
  (bind _returnvalue (Transformation|GetWorldLocation _defaultsceneroot))
  (Transformation|SetActorRotation "0,90.000000, 0")
  (Transformation|SetWorldLocation _defaultsceneroot (Math|Vector|MakeVector (.x _returnvalue) (.y _returnvalue) (Variables|Default|GetHeight)) false false))