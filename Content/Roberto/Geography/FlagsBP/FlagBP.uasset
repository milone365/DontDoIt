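; FlagBP is a flag Blueprint in the Geography content that exposes grab, hint and item-type query functions, apparently from a shared grabbable-item interface.
; All of these are default stubs: it reports neither grabbed nor ready to be grabbed, returns no grab box or rope, and gives empty hint text.
; The construction script is empty, and the graphs hold no flag-specific logic.
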(fn ConstructionScript)

(fn GetGrabBox
  (return 0))

(fn GetHintButtonIcon
  (return "NewEnumerator0"))

(fn GetHintUIText
  (return ""))

(fn GetItemType
  (return "NewEnumerator0"))

(fn GetRope
  (return 0))

(fn IsGrabbed?
  (return false))

(fn ReadytobeGrabbed?
  (return false))