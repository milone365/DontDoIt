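; CountryBP is a country target in a flag-matching geography game that checks FlagObjectBP actors overlapping its box against its Nation.
; A match deactivates the flag, reveals the child actor, removes the particle, plays a checkpoint sound and shows the nation name.
; A mismatch respawns a copy at the flag's start position, destroys the original and calls the player's HurtMessage with effects.
; Both outcomes clear the player's HaveWeight; delays throttle retries.
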(event OnComponentBeginOverlap(Box)
  (params (OverlappedComponent :type Primitive%20Component%20Object%20Reference) (OtherActor :type Actor%20Object%20Reference) (OtherComp :type Primitive%20Component%20Object%20Reference) (OtherBodyIndex :type Integer) (bFromSweep :type Boolean) (SweepResult :type Hit%20Result%20Structure%20%28by%20ref%29))
  (bind _asflag_object_bp (Utilities|Casting|CastToFlagObjectBP OtherActor))
  (bind _output_get (Variables|Default|Setcurrentflag _asflag_object_bp))
  (Utilities|IsValid _output_get
    (:Is%20Valid
      (if (not (Variables|Default|GetIsActived))
        (if (Utilities|Enum|Equal(Enum) (Variables|/Game/Roberto/Geography/FlagObjectBP.FlagObjectBP_C|GetNation (Variables|Default|Getcurrentflag)) (Variables|Default|GetNation))
          (Default|Deactivation (Variables|Default|Getcurrentflag))
          (Utilities|FlowControl|Delay 0.25)
          (CallFunction|Makevisible)
          (elif (not (Variables|Default|Getgenerating))
            (Variables|Default|Setgenerating true)
            (CallFunction|GenerateClone)
            (Utilities|FlowControl|Delay 0.5)
            (Actor|DestroyActor (Variables|Default|Getcurrentflag))
            (Variables|/Game/OuKanu/Character/BP_Character.BP_Character_C|SetHaveWeight (Variables|Default|Getplayer_actor) false)
            (Utilities|FlowControl|Delay 2.0)
            (Variables|Default|Setgenerating false)))))))

(event Custom|Makevisible
  (bind _player_actor (Variables|Default|Getplayer_actor))
  (Audio|SpawnSoundatLocation "/Game/Roberto/AudioManager/Music/SFX_Cue/checkpoint_Cue.checkpoint_Cue" (Transformation|GetWorldLocation (Variables|Default|GetPivot)) "0, 0, 0" 1.0 1.0 0.0 0 0)
  (Rendering|SetVisibility (Variables|Default|GetChildActor) true false)
  (Components|DestroyComponent (Variables|Default|GetParticleSystem))
  (Utilities|IsValid _player_actor
    (:Is%20Valid
      (Variables|/Game/OuKanu/Character/BP_Character.BP_Character_C|SetHaveWeight _player_actor false)
      (Variables|Default|SetIsActived true)
      (Default|SetText (Variables|Default|Getwidget) (Utilities|String|EnumtoString (Variables|Default|GetNation))))))

(event EventBeginPlay
  (bind _returnvalue (Actor|GetActorOfClass "/Game/OuKanu/Character/BP_Player.BP_Player_C"))
  (Variables|Default|Setplayer_actor _returnvalue))

(event Collision|EventActorBeginOverlap
  (params (OtherActor :type Actor%20Object%20Reference)))

(event EventTick
  (params (DeltaSeconds :type Float%20%28single-precision%29)))

(fn ConstructionScript)

(fn GenerateClone
  (bind _currentflag (Variables|Default|Getcurrentflag))
  (bind _defaultsceneroot (Variables|Default|GetDefaultSceneRoot))
  (bind _returnvalue (Transformation|GetWorldLocation _defaultsceneroot))
  (Audio|SpawnSoundatLocation "/Game/OuKanu/Sounds/Stone/Dirt_Explosion_8.Dirt_Explosion_8" _returnvalue "0, 0, 0" 1.0 1.0 0.0 0 0)
  (bind _returnvalue_2 (Game|SpawnActorfromClass "/Game/Roberto/Geography/FlagObjectBP.FlagObjectBP_C" (Math|Transform|MakeTransform (Variables|/Game/Roberto/Geography/FlagObjectBP.FlagObjectBP_C|GetstartPos _currentflag) "0,90.000000, 0" "1.500000,0.500000,1.500000") "Undefined" 0 0))
  (Variables|Default|SetnewFlag _returnvalue_2)
  (Variables|/Game/Roberto/Geography/FlagObjectBP.FlagObjectBP_C|SetNation (Variables|Default|GetnewFlag) (Variables|/Game/Roberto/Geography/FlagObjectBP.FlagObjectBP_C|GetNation _currentflag))
  (Default|SetRelativeFlag (Variables|Default|GetnewFlag))
  (Default|Poseflag (Variables|Default|GetnewFlag))
  (Class|BPICharacter|Hurt(Message) (Variables|Default|Getplayer_actor) 5e+01)
  (Effects|SpawnEmitteratLocation "/Game/OuKanu/FX/FXVarietyPack/Particles/P_ky_hit1.P_ky_hit1" _returnvalue "0, 0, 0" "3.000000,3.000000,3.000000"))