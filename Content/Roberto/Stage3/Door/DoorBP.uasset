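; Level exit door that sends the player to the next level once it is open.
; OpenDoor, callable as an event or run at BeginPlay when IsOpen is set, plays a sound, blacks out the closed door, reveals the open door and sets the Open flag.
; A box overlap by BP_Player while Open loads the level named in Nextlevel.
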(event OnComponentBeginOverlap(Box)
  (params (OverlappedComponent :type Primitive%20Component%20Object%20Reference) (OtherActor :type Actor%20Object%20Reference) (OtherComp :type Primitive%20Component%20Object%20Reference) (OtherBodyIndex :type Integer) (bFromSweep :type Boolean) (SweepResult :type Hit%20Result%20Structure%20%28by%20ref%29))
  (bind _asbp_player (Utilities|Casting|CastToBP_Player OtherActor))
  (Utilities|IsValid _asbp_player
    (:Is%20Valid
      (if (Variables|Default|Getopen)
        (Game|OpenLevel(byName) (Utilities|String|StringToName (Variables|Default|Getnextlevel)))))))

(event Custom|OpenDoor
  (Audio|PlaySound2D "/Game/Roberto/Stage3/MusicQuest/open_door_1.open_door_1" 1.0 1.0 0.0 0 0)
  (Rendering|Material|SetMaterial (Variables|Default|GetDoorClosed) 0 "/Game/Duarte/DuarteResources/DuarteMaterials/Black.Black")
  (Rendering|SetVisibility (Variables|Default|GetDoorOpen) true false)
  (Variables|Default|Setopen true))

(event EventBeginPlay
  (if (Variables|Default|GetIsOpen)
    (CallFunction|OpenDoor)))

(fn ConstructionScript)