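; Puzzle manager for the Stage 3 bath enigma, coordinating the water state of the Lavel actors in the level.
; On BeginPlay it registers itself with every Lavel and splits them by ID into middle and front rows.
; ResetLine stores the passed index as CurrentActive and picks the matching row.
; DeactivateAll then calls WaterOnOff(true) on every Lavel in that row, including any matching the stored index.
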(event Custom|ResetLine
  (params (NewParam :type Integer))
  (Utilities|FlowControl|Sequence
    (:then_0
      (Variables|Default|SetCurrentActive NewParam)
      (if (>= NewParam 4)
        (CallFunction|DeactivateAll (Variables|Default|GetLavelsFront))
        (else
          (CallFunction|DeactivateAll (Variables|Default|GetLavels_Middle)))))))

(event EventBeginPlay
  (bind _outactors (Actor|GetAllActorsOfClass "/Game/Roberto/Stage3/Bath/Enigma/Lavel.Lavel_C"))
  (for _array_element _outactors
    (Default|SetEnigma _array_element self)
    (if (<= (Variables|/Game/Roberto/Stage3/Bath/Enigma/Lavel.Lavel_C|GetID _array_element) 3)
      (Utilities|Array|Add (Variables|Default|GetLavels_Middle) _array_element)
      (else
        (Utilities|Array|Add (Variables|Default|GetLavelsFront) _array_element)))))

(fn ConstructionScript)

(fn DeactivateAll
  (params (Lista :type Array%20of%20Lavel%20Object%20References))
  (for _array_element Lista
    (Default|WateronOff _array_element true)))