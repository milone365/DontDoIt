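; WretchBP is a hand-held tool for the Bath enigma in Stage 3 that operates Lavel actors.
; Each tick it snaps its root to the RightHandLocation of a BP_Player found on BeginPlay.
; A box overlap stores the Lavel and raises an in-zone flag, rechecked every second until the overlap ends.
; While in zone, holding Y or the gamepad top face button calls UseWretch on that Lavel every tick.
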(event OnComponentBeginOverlap(Box)
  (params (OverlappedComponent :type Primitive%20Component%20Object%20Reference) (OtherActor :type Actor%20Object%20Reference) (OtherComp :type Primitive%20Component%20Object%20Reference) (OtherBodyIndex :type Integer) (bFromSweep :type Boolean) (SweepResult :type Hit%20Result%20Structure%20%28by%20ref%29))
  (bind _aslavel (Utilities|Casting|CastToLavel OtherActor))
  (Utilities|IsValid _aslavel
    (:Is%20Valid
      (Variables|Default|SetcurrentLavel _aslavel)
      (Variables|Default|SetInzone true)
      (Utilities|FlowControl|Delay 1.0 :!label _label)
      (if (Collision|IsOverlappingActor (Variables|Default|GetBox) OtherActor :!class /Script/Engine.PrimitiveComponent)
        (goto _label)
        (else
          (Variables|Default|SetInzone false))))))

(event EventTick
  (params (DeltaSeconds :type Float%20%28single-precision%29))
  (bind _returnvalue (Game|GetPlayerController 0))
  (bind _player (Variables|Default|GetPlayer))
  (bind _defaultsceneroot (Variables|Default|GetDefaultSceneRoot))
  (bind _righthandlocation (Variables|/Game/OuKanu/Character/BP_Character.BP_Character_C|GetRightHandLocation _player))
  (Utilities|FlowControl|Sequence
    (:then_0
      (Utilities|IsValid _player
        (:Is%20Valid
          (Transformation|SetWorldLocation _defaultsceneroot (Transformation|GetWorldLocation _righthandlocation) false false)
          (Transformation|SetWorldRotation _defaultsceneroot (Transformation|GetWorldRotation _righthandlocation) false false))))
    (:then_1
      (if (Variables|Default|GetInzone)
        (if (or (Game|Player|IsInputKeyDown _returnvalue "Gamepad_FaceButton_Top") (Game|Player|IsInputKeyDown _returnvalue "Y"))
          (Default|UseWretch (Variables|Default|GetcurrentLavel)))))))

(event EventBeginPlay
  (bind _returnvalue (Actor|GetActorOfClass "/Game/OuKanu/Character/BP_Player.BP_Player_C"))
  (Variables|Default|SetPlayer _returnvalue))

(fn ConstructionScript)

(fn SetPlayer
  (params (NewParam :type BP%20Player%20Object%20Reference))
  (CallFunction|SetPlayer NewParam))