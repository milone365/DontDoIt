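; Stage 3 gate Blueprint that slides its static mesh between a left point, a right point and its starting position.
; It caches the mesh's relative location on BeginPlay, and three events drive MoveComponentTo toward each target.
; MoveLeft and MoveBack use the Speed variable as move duration, while MoveRight does not.
; Each move passes the mesh's world rotation as the relative target rotation.
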(event Custom|MoveRight
  (Components|MoveComponentTo (Variables|Default|GetStaticMesh) (Variables|/Script/Engine.SceneComponent|GetRelativeLocation (Variables|Default|GetrightPoint)) (Transformation|GetWorldRotation (Variables|Default|GetStaticMesh)) false false 0.2 false))

(event Custom|MoveLeft
  (Components|MoveComponentTo (Variables|Default|GetStaticMesh) (Variables|/Script/Engine.SceneComponent|GetRelativeLocation (Variables|Default|GetLeftPoint)) (Transformation|GetWorldRotation (Variables|Default|GetStaticMesh)) false false (Variables|Default|Getspeed) false))

(event Custom|MoveBack
  (Components|MoveComponentTo (Variables|Default|GetStaticMesh) (Variables|Default|GetDefaultPos) (Transformation|GetWorldRotation (Variables|Default|GetStaticMesh)) false false (Variables|Default|Getspeed) false))

(event EventBeginPlay
  (Variables|Default|SetDefaultPos (Variables|/Script/Engine.SceneComponent|GetRelativeLocation (Variables|Default|GetStaticMesh))))

(fn ConstructionScript)