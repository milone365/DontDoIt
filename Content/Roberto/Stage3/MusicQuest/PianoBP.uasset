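; PianoBP is the piano trigger for a music quest that opens a door after three completed melodies.
; On first player overlap it shows MusicQuest_Widget with UI-only input, stops background music and presents a melody.
; Wrong results re-show the problem after a delay, while completions play that track and advance.
; The last success restores game input and opens DoorBP; GrateUp is an empty stub, its grate-raising logic unconnected.
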(event OnComponentBeginOverlap(Box)
  (params (OverlappedComponent :type Primitive%20Component%20Object%20Reference) (OtherActor :type Actor%20Object%20Reference) (OtherComp :type Primitive%20Component%20Object%20Reference) (OtherBodyIndex :type Integer) (bFromSweep :type Boolean) (SweepResult :type Hit%20Result%20Structure%20%28by%20ref%29))
  (bind _returnvalue (Game|GetPlayerController 0))
  ;[1 1 1] TRIGGER
  (bind _asbp_player (Utilities|Casting|CastToBP_Player OtherActor))
  (Utilities|IsValid _asbp_player
    (:Is%20Valid
      (if (not (Variables|Default|GetActivate))
        (Variables|Default|SetActivate true)
        (bind _returnvalue_2 (UserInterface|CreateWidget "/Game/Roberto/Stage3/MusicQuest/MusicQuest_Widget.MusicQuest_Widget_C"))
        (bind _output_get (Variables|Default|SetMusicWidget _returnvalue_2))
        (UserInterface|Viewport|AddtoViewport _output_get 0)
        (Input|SetInputModeUIOnly _returnvalue (Variables|/Game/Roberto/Stage3/MusicQuest/MusicQuest_Widget.MusicQuest_Widget_C|GetButton_193 (Variables|Default|GetMusicWidget)) "DoNotLock")
        (Variables|/Script/Engine.PlayerController|SetbShowMouseCursor _returnvalue true)
        (bind _returnvalue_3 (Actor|GetActorOfClass "/Game/Roberto/AudioManager/AudioManager.AudioManager_C"))
        (bind _output_get_2 (Variables|Default|Setaudio_manager _returnvalue_3))
        (Audio|Components|Audio|Stop (Variables|/Game/Roberto/AudioManager/AudioManager.AudioManager_C|GetBGM _output_get_2))
        (CallFunction|BuildProblem)))))

(event Custom|CompleteMusic
  (bind _audio_manager (Variables|Default|Getaudio_manager))
  ;[1 1 1] ONTAKING RESULT
  (Default|StopMusic _audio_manager)
  (Default|PlayThisSound _audio_manager (Utilities|Array|Get(acopy) (Variables|Default|GetMusicList) (Variables|Default|GetcompletingIndex)))
  (CallFunction|GrateUp)
  (bind _output_get (Variables|Default|SetcompletingIndex (+ (Variables|Default|GetcompletingIndex) 1)))
  (if (>= _output_get 3)
    (CallFunction|OpenDoor)
    (else
      (CallFunction|OpenRoute))))

(event Custom|OpenRoute
  (Utilities|FlowControl|Delay 15.0)
  (Default|StopMusic (Variables|Default|Getaudio_manager))
  (CallFunction|BuildProblem))

(event Custom|OpenDoor
  (Input|SetInputModeGameOnly (Game|GetPlayerController 0))
  (Widget|RemovefromParent (Variables|Default|GetMusicWidget))
  (bind _returnvalue (Actor|GetActorOfClass "/Game/Roberto/Stage3/Door/DoorBP.DoorBP_C"))
  (Utilities|IsValid _returnvalue
    (:Is%20Valid
      (Default|OpenDoor _returnvalue))))

(event Custom|BuildProblem
  ;[1 1 1] Build
  (Default|ShowProblem (Variables|Default|GetMusicWidget) (Utilities|Array|Get(acopy) (Variables|Default|GetMusic) (Variables|Default|GetcompletingIndex)) self))

(event Custom|WrongResult
  (Utilities|FlowControl|Delay 2.0)
  ;[1 1 1] Build
  (Default|ShowProblem (Variables|Default|GetMusicWidget) (Utilities|Array|Get(acopy) (Variables|Default|GetMusic) (Variables|Default|GetcompletingIndex)) self))

(fn ConstructionScript)

(fn GrateUp)