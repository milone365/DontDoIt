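; Battery switch point for Stage 3 that takes an overlapping BP_Battery and reports its activation to the quest.
; ActivationCheck casts the overlapping actor and uses the Actived flag to return a battery only once.
; The overlap handler destroys that battery and the Cube component, then reveals the switch's own battery mesh.
; It passes PointIndex to the GrountQuestController found at BeginPlay and plays a checkpoint sound.
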(event OnComponentBeginOverlap(Box)
  (params (OverlappedComponent :type Primitive%20Component%20Object%20Reference) (OtherActor :type Actor%20Object%20Reference) (OtherComp :type Primitive%20Component%20Object%20Reference) (OtherBodyIndex :type Integer) (bFromSweep :type Boolean) (SweepResult :type Hit%20Result%20Structure%20%28by%20ref%29))
  (bind _questcontroller (Variables|Default|GetquestController))
  (bind _asbp_battery (|ActivationCheck OtherActor))
  (Actor|DestroyActor _asbp_battery)
  (Components|DestroyComponent (Variables|Default|GetCube))
  (Rendering|SetVisibility (Variables|Default|Getbatterymesh) true false)
  (Utilities|IsValid _questcontroller
    (:Is%20Valid
      (Default|OnPointActivation _questcontroller (Variables|Default|GetPoint_index))
      (Audio|SpawnSoundatLocation "/Game/Roberto/AudioManager/Music/tracks/checkpoint.checkpoint" (Variables|/Script/Engine.SceneComponent|GetRelativeLocation (Variables|Default|Getbatterymesh)) "0, 0, 0" 1.0 1.0 0.0 0 0))))

(event EventBeginPlay
  (bind _returnvalue (Actor|GetActorOfClass "/Game/Roberto/Stage3/GrountQuestController.GrountQuestController_C"))
  (Variables|Default|SetquestController _returnvalue))

(fn ConstructionScript)