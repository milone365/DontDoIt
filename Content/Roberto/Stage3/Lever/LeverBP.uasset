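; LeverBP is a lever that toggles the level's gate whenever BP_Player overlaps its box.
; BeginPlay finds the gate with GetActorOfClass, so the lever drives whichever GateBP that lookup returns.
; Each overlap flips Closed and swaps the open and closed lever meshes.
; Opening moves the gate left or right according to MoveLeft, and closing calls the gate's MoveBack.
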(event OnComponentBeginOverlap(Box)
  (params (OverlappedComponent :type Primitive%20Component%20Object%20Reference) (OtherActor :type Actor%20Object%20Reference) (OtherComp :type Primitive%20Component%20Object%20Reference) (OtherBodyIndex :type Integer) (bFromSweep :type Boolean) (SweepResult :type Hit%20Result%20Structure%20%28by%20ref%29))
  (bind _asbp_player (Utilities|Casting|CastToBP_Player OtherActor))
  (Utilities|IsValid _asbp_player
    (:Is%20Valid
      (if (Variables|Default|GetClosed)
        (Variables|Default|SetClosed false)
        (CallFunction|OpenGate)
        (else
          (Variables|Default|SetClosed true)
          (CallFunction|CloseGate))))))

(event Custom|OpenGate
  (Rendering|SetVisibility (Variables|Default|GetOpenMesh) true false)
  (Rendering|SetVisibility (Variables|Default|GetCloseMesh) false false)
  (if (Variables|Default|GetMoveLeft)
    (Default|MoveLeft (Variables|Default|GetGate))
    (else
      (Default|MoveRight (Variables|Default|GetGate)))))

(event Custom|CloseGate
  (Rendering|SetVisibility (Variables|Default|GetOpenMesh) false false)
  (Rendering|SetVisibility (Variables|Default|GetCloseMesh) true false)
  (Default|MoveBack (Variables|Default|GetGate)))

(event EventBeginPlay
  (bind _returnvalue (Actor|GetActorOfClass "/Game/Roberto/Stage3/Gate/GateBP.GateBP_C"))
  (Variables|Default|SetGate _returnvalue))

(fn ConstructionScript)