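; Quest actor that starts a multiplication quiz when the player first overlaps its box and opens a door once it is solved.
; It generates random products, shows them in a MathWidget with UI-only input, and checks replies passed to CheckResult as strings.
; Wrong answers drop a random SpikeWallBP and show an error through ErrorWidget.
; Three correct answers restore game input, open the DoorBP and destroy the actor.
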(event OnComponentBeginOverlap(Box)
  (params (OverlappedComponent :type Primitive%20Component%20Object%20Reference) (OtherActor :type Actor%20Object%20Reference) (OtherComp :type Primitive%20Component%20Object%20Reference) (OtherBodyIndex :type Integer) (bFromSweep :type Boolean) (SweepResult :type Hit%20Result%20Structure%20%28by%20ref%29))
  (if (not (Variables|Default|Getresolved))
    (Variables|Default|Setresolved true)
    (bind _asbp_player (Utilities|Casting|CastToBP_Player OtherActor))
    (Utilities|IsValid _asbp_player
      (:Is%20Valid
        (CallFunction|StartQuestion)))))

(event Custom|CheckResult
  (params (Reply :type String))
  ;[1 1 1] CLEARCHECK
  (if (Utilities|Enum|Equal(Enum) Reply (Utilities|String|JoinStringArray (Utilities|Array|MakeArray (Utilities|String|ToString(Integer) (Variables|Default|Getresult))) ","))
    (bind _output_get (Variables|Default|Setclearproblem (+ (Variables|Default|Getclearproblem) 1)))
    (if (>= _output_get 3)
      (Default|ShowClear (Variables|Default|GeterrorLog))
      (CallFunction|QuestClear)
      (else
        (Default|ShowCorrect (Variables|Default|GeterrorLog))
        (Utilities|Build)))
    (else
      (CallFunction|Fall))))

(event Custom|QuestClear
  ;[1 1 1] EndQuest
  (Widget|RemovefromParent (Variables|Default|GetM_Widget))
  (Input|SetInputModeGameOnly (Game|GetPlayerController 0))
  (CallFunction|OpenDoor)
  (Actor|DestroyActor))

(event Custom|StartQuestion
  (bind _returnvalue (Game|GetPlayerController 0))
  ;[1 1 1] Start
  (CallFunction|RandomProblem)
  (bind _returnvalue_2 (UserInterface|CreateWidget "/Game/Roberto/QUEST/MathWidget.MathWidget_C"))
  (bind _output_get (Variables|Default|SetM_Widget _returnvalue_2))
  (UserInterface|Viewport|AddtoViewport _output_get 0)
  (Default|BuildProblem (Variables|Default|GetM_Widget) (Variables|Default|GetNum1) (Variables|Default|GetNum2) self)
  (Input|SetInputModeUIOnly _returnvalue (Variables|/Game/Roberto/QUEST/MathWidget.MathWidget_C|GetButton_233 (Variables|Default|GetM_Widget)) "DoNotLock")
  (Variables|/Script/Engine.PlayerController|SetbShowMouseCursor _returnvalue true)
  (bind _returnvalue_3 (UserInterface|CreateWidget "/Game/Roberto/QUEST/ErrorWidget.ErrorWidget_C"))
  (bind _output_get_2 (Variables|Default|SeterrorLog _returnvalue_3))
  (UserInterface|Viewport|AddtoViewport _output_get_2 0))

(event Custom|RandomProblem
  ;[1 1 1] MakeRandomProblem
  (bind _output_get (Variables|Default|SetNum1 (Math|Random|RandomIntegerinRange 2 20)))
  (bind _output_get_2 (Variables|Default|SetNum2 (Math|Random|RandomIntegerinRange 2 20)))
  (Variables|Default|Setresult (* _output_get _output_get_2)))

(event Custom|OpenDoor
  (bind _returnvalue (Actor|GetActorOfClass "/Game/Roberto/Stage3/Door/DoorBP.DoorBP_C"))
  (Utilities|IsValid _returnvalue
    (:Is%20Valid
      (Default|OpenDoor _returnvalue))))

(event Custom|Fall
  (Default|ShowError (Variables|Default|GeterrorLog))
  (Default|Fall (Utilities|Array|Get(acopy) (Variables|Default|Getwalls) (Math|Random|RandomIntegerinRange 0 (- (Utilities|Array|Length (Variables|Default|Getwalls)) 1)))))

(event EventBeginPlay
  (bind _outactors (Actor|GetAllActorsOfClass "/Game/Roberto/Stage3/Trap/SpikeWallBP.SpikeWallBP_C"))
  (Variables|Default|Setwalls _outactors))

(fn ConstructionScript)